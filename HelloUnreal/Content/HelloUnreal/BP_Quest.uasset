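; BP_Quest is a string-parsing test Blueprint that prints the dot-separated segments of its Strings variable.
; Each Tick splits off the leading segment, prints it and stores the remainder back in Strings, spreading the loop across frames.
; When no dot remains, it prints the final segment and later Ticks do nothing.
; Disconnected nodes hold earlier experiments with nested Split chains and a literal-string Split result check.
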(event `self.ReceiveTick`
  (params (DeltaSeconds :type "Float (single-precision)"))
  (bind (_lefts _rights _returnvalue) (`KismetStringLibrary.Split` (`self.Strings`) "."))
  (if _returnvalue
    (`KismetSystemLibrary.PrintString` _lefts)
    (set `self.Strings` _rights)
    (if (not (`.ReturnValue` (`KismetStringLibrary.Split` (`self.Strings`) ".")))
      (`KismetSystemLibrary.PrintString` (`self.Strings`)))))

(fn `UserConstructionScript`)